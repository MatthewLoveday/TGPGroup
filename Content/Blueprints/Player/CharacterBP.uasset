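; Player character for a 3D platformer, with camera-relative movement, stomp kills on enemies when airborne, death otherwise, and safety-net respawn.
; Tick branches on MoveSet: default adds faster falling and an air dive, balloon makes Dive inflate the head for lift until overinflation kills.
; Both share trace-based wall slides feeding wall jumps and a ground-approach check; helicopter handlers are empty.
; Dynamic body and mouth materials show inflation through red tinting and flashing.
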(event OnComponentBeginOverlap(LeftFoot)
  (params (OverlappedComponent :type Primitive%20Component%20Object%20Reference) (OtherActor :type Actor%20Object%20Reference) (OtherComp :type Primitive%20Component%20Object%20Reference) (OtherBodyIndex :type Integer) (bFromSweep :type Boolean) (SweepResult :type Hit%20Result%20Structure%20%28by%20ref%29))
  (bind _footsmoke (Variables|Default|GetFootSmoke))
  ;[1 1 1] Feet Smoke
  (Components|Activation|Activate _footsmoke true)
  (Utilities|FlowControl|Delay 0.2)
  (Components|Activation|Deactivate _footsmoke))

(event OnComponentBeginOverlap(RightFoot)
  (params (OverlappedComponent :type Primitive%20Component%20Object%20Reference) (OtherActor :type Actor%20Object%20Reference) (OtherComp :type Primitive%20Component%20Object%20Reference) (OtherBodyIndex :type Integer) (bFromSweep :type Boolean) (SweepResult :type Hit%20Result%20Structure%20%28by%20ref%29))
  (bind _footsmoke (Variables|Default|GetFootSmoke))
  ;[1 1 1] Feet Smoke
  (Components|Activation|Activate _footsmoke true)
  (Utilities|FlowControl|Delay 0.2)
  (Components|Activation|Deactivate _footsmoke))

(event EventTick
  (params (DeltaSeconds :type Float%20%28single-precision%29))
  (bind _moveset (Variables|Default|GetmoveSet))
  (bind _boytint (Variables|HeadInflation|GetBoyTint))
  ;[1 1 1] Default Moveset Tick
  (Rendering|Material|SetVectorParameterValue (Variables|HeadInflation|GetBodyMat) "Tint" _boytint :!class /Script/Engine.MaterialInstanceDynamic)
  (Rendering|Material|SetVectorParameterValue (Variables|HeadInflation|GetMouth%20Mat) "Tint" _boytint :!class /Script/Engine.MaterialInstanceDynamic)
  (AnimVariables|UpdateAnimVariables)
  (Debug|DebugDrawMovement (Utilities|DrawDebug))
  (if (Class|PlatformerGameCharacter|IsAlive)
    (switch Utilities|FlowControl|Switch|SwitchonEMovesetEnum _moveset
      (:M_Default
        (WallJump|PerformWallChecks)
        (CallFunction|DetermineifGroundApproach 4e+02)
        (CallFunction|PerformBetterJump)
        (Variables|/Script/Engine.CharacterMovementComponent|SetbOrientRotationToMovement (Variables|Character|GetCharacterMovement) (not (AI|Components|NavMovement|IsFalling (Variables|Character|GetCharacterMovement))))
        (Dive|PerformEndDiveChecks))
      (:M_Balloon
        (WallJump|PerformWallChecks)
        (CallFunction|DetermineifGroundApproach 4e+02)
        (bind _headinflation (CallFunction|HandleHeadInflation))
        (if (> _headinflation (Variables|HeadInflation|GetMaxHeadInflation))
          (CallFunction|Die))))
    (elif (Utilities|Enum|Equal(Enum) _moveset "M_Balloon")
      (Variables|HeadInflation|SetHeadInflation -1e+02))))

(event EventEnterBalloonMoveSet
  ;[1 1 1] Entry and Exit Conditions
  (Rendering|Components|TextRender|SetText (Variables|/Game/Blueprints/HUD/ControlHintWidget.ControlHintWidget_C|GetHint (Variables|/Game/Blueprints/HUD/ControlHintScreen.ControlHintScreen_C|GetControlHintWidget (Variables|Default|Gethintscreen))) "Inflate"))

(event EventEnterDefaultMoveSet
  ;[1 1 1] Entry and Exit Conditions
  (Variables|/Script/Engine.CharacterMovementComponent|SetGravityScale (Variables|Character|GetCharacterMovement) 3.0) ; Reset the gravity scale
  (Variables|HeadInflation|SetHeadInflation 0.0)
  (Variables|HeadInflation|SetHeadInflation 0.0)
  (Rendering|Components|TextRender|SetText (Variables|/Game/Blueprints/HUD/ControlHintWidget.ControlHintWidget_C|GetHint (Variables|/Game/Blueprints/HUD/ControlHintScreen.ControlHintScreen_C|GetControlHintWidget (Variables|Default|Gethintscreen))) "Dive"))

(event EventEnterHeliMoveSet
  ;[1 1 1] Entry and Exit Conditions
)

(event EventExitBalloonMoveSet
  ;[1 1 1] Entry and Exit Conditions
)

(event EventExitDefaultMoveSet
  ;[1 1 1] Entry and Exit Conditions
  (Variables|HeadInflation|SetHeadInflation 0.0))

(event EventExitHeliMoveSet
  ;[1 1 1] Entry and Exit Conditions
)

(event EventBeginPlay
  (bind _mesh (Variables|Character|GetMesh))
  ;[1 1 1] Add UI
  (bind _returnvalue (UserInterface|CreateWidget "/Game/Blueprints/HUD/ControlHintScreen.ControlHintScreen_C"))
  (UserInterface|Viewport|AddtoViewport _returnvalue 0)
  (Variables|Default|Sethintscreen _returnvalue)
  (bind _returnvalue_2 (Rendering|Material|CreateDynamicMaterialInstance _mesh 0 "/Game/Models/Characters/Boy/BoyBodyMatInstance.BoyBodyMatInstance" "Body" :!class /Script/Engine.PrimitiveComponent))
  (Variables|HeadInflation|SetBodyMat _returnvalue_2)
  (bind _returnvalue_3 (Rendering|Material|CreateDynamicMaterialInstance _mesh 1 "/Game/Models/Characters/Boy/BoyEyesMatInstance.BoyEyesMatInstance" "Mouth" :!class /Script/Engine.PrimitiveComponent))
  (Variables|HeadInflation|SetMouth%20Mat _returnvalue_3)
  (switch Utilities|FlowControl|Switch|SwitchonEMovesetEnum (Variables|Default|GetmoveSet)))

(event EventRespawn
  ;[1 1 1] respawn
  (Transformation|Teleport (Variables|/Script/tgp.PlatformerGameSafetyNet|GetTeleportLocation (Variables|Default|GetSafetyNetRef)) "0, 0, 0")
  (Variables|Default|Setalive true)
  (Variables|HeadInflation|SetHeadInflation 0.0))

(event Collision|EventHit
  (params (MyComp :type Primitive%20Component%20Object%20Reference) (Other :type Actor%20Object%20Reference) (OtherComp :type Primitive%20Component%20Object%20Reference) (bSelfMoved :type Boolean) (HitLocation :type Vector :default "0, 0, 0") (HitNormal :type Vector :default "0, 0, 0") (NormalImpulse :type Vector :default "0, 0, 0") (Hit :type Hit%20Result%20Structure%20%28by%20ref%29))
  ;[1 1 1] Enemy Interaction
  (bind _asenemy_base_character (Utilities|Casting|CastToEnemyBaseCharacter Other))
  (if (Variables|/Script/tgp.EnemyBaseCharacter|GetAlive _asenemy_base_character)
    (if (AI|Components|NavMovement|IsFalling (Variables|Character|GetCharacterMovement))
      (Class|EnemyBaseCharacter|Die _asenemy_base_character)
      (else
        (CallFunction|Die)))
    (Audio|PlaySoundatLocation 0 HitLocation "0, 0, 0" 1.0 1.0 0.0 0 0 0)))

(event Input|ActionEvents|InputActionJump
  (params (Key :type Key%20Structure))
  ;[1 1 1] Perform Jump
  (:Pressed
    (if (Class|PlatformerGameCharacter|IsAlive)
      (switch Utilities|FlowControl|Switch|SwitchonEMovesetEnum (Variables|Default|GetmoveSet) ; Pressed
        (:M_Default
          _)
        (:M_Helicopter
          _)
        (:M_Balloon
          _))
      (if (not (Variables|Default|GetLockJump))
        (if (Variables|WallJump|GetIsOnWall)
          (WallJump|JumpOffWall)
          (else
            (Character|Jump))))))
  (:Released
    (switch Utilities|FlowControl|Switch|SwitchonEMovesetEnum (Variables|Default|GetmoveSet) ; Released
      (:M_Default
        _)
      (:M_Helicopter
        _)
      (:M_Balloon
        _))
    (Character|StopJumping)))

(event Input|ActionEvents|InputActionDive
  (params (Key :type Key%20Structure))
  (bind _footsmoke (Variables|Default|GetFootSmoke))
  ;[1 1 1] Special Move
  (:Pressed
    (if (Class|PlatformerGameCharacter|IsAlive)
      (switch Utilities|FlowControl|Switch|SwitchonEMovesetEnum (Variables|Default|GetmoveSet) ; Pressed
        (:M_Default
          (Dive|TryBeginDive))
        (:M_Balloon
          (Variables|HeadInflation|SetHeadInflation (+ (Variables|HeadInflation|GetHeadInflation) 2e+01))
          (Character|LaunchCharacter "0, 0,1000.000000" false true)
          (Components|Activation|Activate _footsmoke true)
          (Utilities|FlowControl|Delay 0.2)
          (Components|Activation|Deactivate _footsmoke)))))
  (:Released
    (switch Utilities|FlowControl|Switch|SwitchonEMovesetEnum (Variables|Default|GetmoveSet)) ; Released
  ))

(event Input|AxisEvents|InputAxisForwardMovement
  (params (AxisValue :type Float%20%28single-precision%29))
  ;[1 1 1] Basic Movement
  (if (not (or (Variables|Default|GetLockMovement) (not (Class|PlatformerGameCharacter|IsAlive))))
    (Pawn|Input|AddMovementInput (Math|Vector|GetForwardVector (Math|Rotator|MakeRotator 0.0 0.0 (.Yaw (Math|Rotator|BreakRotator (Pawn|GetControlRotation :!class /Script/Engine.Pawn))))) AxisValue false)))

(event Input|AxisEvents|InputAxisHorizontalMovement
  (params (AxisValue :type Float%20%28single-precision%29))
  ;[1 1 1] Basic Movement
  (if (not (or (Variables|Default|GetLockMovement) (not (Class|PlatformerGameCharacter|IsAlive))))
    (Pawn|Input|AddMovementInput (Math|Vector|GetRightVector (Math|Rotator|MakeRotator 0.0 0.0 (.Yaw (Math|Rotator|BreakRotator (Pawn|GetControlRotation :!class /Script/Engine.Pawn))))) AxisValue false)))

(event Input|AxisEvents|InputAxisMouseHorizontal
  (params (AxisValue :type Float%20%28single-precision%29))
  ;[1 1 1] Mouse Movement
  (Pawn|Input|AddControllerYawInput AxisValue))

(event Input|AxisEvents|InputAxisMouseVertical
  (params (AxisValue :type Float%20%28single-precision%29))
  ;[1 1 1] Mouse Movement
  (Pawn|Input|AddControllerPitchInput AxisValue))

(fn ConstructionScript)

(fn UpdateAnimVariables
  (Variables|AnimVariables|SetWalking (or (!= (Input|AxisValues|GetForwardMovement) 0.0) (!= (Input|AxisValues|GetHorizontalMovement) 0.0)))
  (return))

(fn EnterWalljump
  (params (WallNormal :type Vector))
  (bind _charactermovement (Variables|Character|GetCharacterMovement))
  (if (not (Variables|WallJump|GetIsOnWall))
    (Variables|WallJump|SetIsOnWall true)
    (Variables|/Script/Engine.CharacterMovementComponent|SetGravityScale _charactermovement 1.0)
    (Variables|WallJump|SetWallNormal (Math|Vector|Normalize WallNormal))
    (Variables|/Script/Engine.MovementComponent|SetVelocity _charactermovement (Math|Vector|MakeVector (.X (Math|Vector|BreakVector (Variables|/Script/Engine.MovementComponent|GetVelocity _charactermovement))) (.Y (Math|Vector|BreakVector (Variables|/Script/Engine.MovementComponent|GetVelocity _charactermovement))) 0.0))
    (Variables|WallJump|SetWallCooldown 0.3)
    (Components|Activation|Activate (Variables|Default|GetWallSmoke) true)
    (Variables|Dive|SetDive false)
    (Audio|Components|Audio|Play (Variables|Default|GetWallslideSound) 0.0)
    (return)))

(fn LeaveWallJump
  (if (Variables|WallJump|GetIsOnWall)
    (Variables|WallJump|SetIsOnWall false)
    (Variables|/Script/Engine.CharacterMovementComponent|SetGravityScale (Variables|Character|GetCharacterMovement) 3.0)
    (Variables|WallJump|SetWallCooldown 0.3)
    (Components|Activation|Deactivate (Variables|Default|GetWallSmoke))
    (Audio|Components|Audio|Stop (Variables|Default|GetWallslideSound))
    (return)))

(fn GetPlayerPushingTowardVector
  (params (Vector :type Vector) (Threshold :type Float%20%28single-precision%29))
  (bind _returnvalue (Transformation|GetVelocity))
  (bind (_x _y) (Math|Vector|BreakVector _returnvalue))
  (return (>= (Math|Vector|DotProduct Vector (Math|Vector|Normalize (+ (Math|Vector|MakeVector _x _y 0.0) (* (VectorHelpers|CalculateMovementVector) 25.0)))) Threshold)))

(fn DebugDrawVelocity
  (params (Length :type Float%20%28single-precision%29) (Draw :type Boolean))
  (bind _returnvalue (Transformation|GetActorLocation))
  (if Draw
    (Rendering|Debug|DrawDebugLine _returnvalue (+ _returnvalue (* (Math|Vector|Normalize (Variables|/Script/Engine.MovementComponent|GetVelocity (Variables|Character|GetCharacterMovement))) Length)) "(R=1.000000,G=0.997690,B=0.962442,A=1.000000)" 0.0 1e+01)
    (return)
    (else
      (return))))

(fn DebugDrawMovement
  (params (Draw :type Boolean))
  (bind _returnvalue (Transformation|GetActorLocation))
  (if Draw
    (Rendering|Debug|DrawDebugLine _returnvalue (+ _returnvalue (* (VectorHelpers|CalculateMovementVector) 2e+02)) "(R=1.000000,G=0.000000,B=0.183393,A=1.000000)" 0.0 1e+01))
  (return))

(fn CalculateMovementVector
  (bind _returnvalue (Pawn|GetControlRotation :!class /Script/Engine.Pawn))
  (bind _yaw (Math|Rotator|BreakRotator _returnvalue))
  (bind _returnvalue_2 (Math|Rotator|MakeRotator 0.0 0.0 _yaw))
  (return (Math|Vector|Normalize (+ (* (Math|Vector|GetForwardVector _returnvalue_2) (Input|AxisValues|GetForwardMovement)) (* (Math|Vector|GetRightVector _returnvalue_2) (Input|AxisValues|GetHorizontalMovement))))))

(fn PerformWallChecks
  ;[1 1 1] If we're next to a wall && not grounded
  (bind _output_get (Variables|WallJump|SetWallCooldown (- (Variables|WallJump|GetWallCooldown) (Utilities|Time|GetWorldDeltaSeconds))))
  (if (<= _output_get 0.0) ; Cooldown to prevent double wall jump
    (if (not (AI|Components|NavMovement|IsFalling (Variables|Character|GetCharacterMovement)))
      (Variables|WallJump|SetWallJumpString? false))
    (Utilities|FlowControl|Sequence
      (:then_0
        (bind _returnvalue (Class|PlatformerGameCharacter|PerformCircleTrace "ECC_GameTraceChannel1" 1e+01 8e+01 (Utilities|DrawDebug)))
        (LocalVariables|SetLWallCollide (.bBlockingHit (Collision|BreakHitResult _returnvalue)))
        (LocalVariables|SetLWallNormal (.ImpactNormal (Collision|BreakHitResult _returnvalue))))
      (:then_1
        (if (LocalVariables|GetLWallCollide)
          (if (!= (.Z (Math|Vector|BreakVector (LocalVariables|GetLWallNormal))) 1.0)
            (if (AI|Components|NavMovement|IsFalling (Variables|Character|GetCharacterMovement)) ; If the character is in the air
              (bind _result (VectorHelpers|GetPlayerPushingTowardVector (Math|Vector|RotateVector (Math|Vector|MakeVector (.X (Math|Vector|BreakVector (LocalVariables|GetLWallNormal))) (.Y (Math|Vector|BreakVector (LocalVariables|GetLWallNormal))) 0.0) "0,180.000000, 0") 0.75))
              (if (or _result (Variables|WallJump|GetWallJumpString?)) ; If character pushing towards wall
                (WallJump|EnterWalljump (Math|Vector|MakeVector (.X (Math|Vector|BreakVector (LocalVariables|GetLWallNormal))) (.Y (Math|Vector|BreakVector (LocalVariables|GetLWallNormal))) 0.0))
                (return true))
              (else
                (WallJump|LeaveWallJump :!label _label)
                (return false)))
            (else
              (goto _label)))
          (else
            (goto _label)))))))

(fn JumpOffWall
  (bind _wallnormal (Variables|WallJump|GetWallNormal))
  (if (Variables|WallJump|GetIsOnWall)
    (WallJump|LeaveWallJump)
    (Character|LaunchCharacter (* (+ _wallnormal "0, 0,2.000000") 8e+02) true true)
    (Transformation|SetActorRotation (Math|Conversions|RotationFromXVector _wallnormal))
    (Variables|WallJump|SetWallJumpString? true)
    (return)))

(fn PerformBetterJump
  (if (<= (.Z (Math|Vector|BreakVector (Variables|/Script/Engine.MovementComponent|GetVelocity (Variables|Character|GetCharacterMovement)))) 0.0)
    (Variables|/Script/Engine.MovementComponent|SetVelocity (Variables|Character|GetCharacterMovement) (+ (Variables|/Script/Engine.MovementComponent|GetVelocity (Variables|Character|GetCharacterMovement)) (* (* (* "0, 0,1.000000" (Components|Movement|GetGravityZ (Variables|Character|GetCharacterMovement))) (- (Variables|Default|GetFallMultiplier) 1.0)) (Utilities|Time|GetWorldDeltaSeconds))))
    (return)))

(fn DetermineifGroundApproach
  (params (Height :type Float%20%28single-precision%29))
  (bind _returnvalue (Transformation|GetActorLocation))
  (if (<= (.Z (Math|Vector|BreakVector (Variables|/Script/Engine.MovementComponent|GetVelocity (Variables|Character|GetCharacterMovement)))) 0.0)
    (bind _returnvalue_2 (Collision|LineTraceByChannel _returnvalue (+ _returnvalue (Math|Vector|MakeVector 0.0 0.0 (- 0.0 Height))) "TraceTypeQuery1" false 0 "None"))
    (Variables|Dive|SetApproachingGround _returnvalue_2)
    (return)
    (else
      (Variables|Dive|SetApproachingGround false)
      (return))))

(fn TryBeginDive
  (bind _out (VectorHelpers|CalculateMovementVector))
  (bind _returnvalue (Pawn|GetControlRotation :!class /Script/Engine.Pawn))
  (bind _returnvalue_2 (Math|Rotator|GetRotationXVector _returnvalue))
  (bind (_x _y) (Math|Vector|BreakVector _out))
  (bind (_x_2 _y_2) (Math|Vector|BreakVector _returnvalue_2))
  (bind _returnvalue_3 (Math|Vector|MakeVector _x _y 0.0))
  (bind _returnvalue_4 (Math|Vector|MakeVector _x_2 _y_2 0.0))
  (if (Math|Boolean|ANDBoolean (AI|Components|NavMovement|IsFalling (Variables|Character|GetCharacterMovement)) (not (Variables|WallJump|GetIsOnWall)) (not (Variables|Dive|GetDive)) (Variables|Dive|GetCanDive))
    (Variables|Dive|SetCanDive false)
    (Variables|Dive|SetDive true)
    (Variables|Default|SetLockMovement true)
    (if (<= (Math|Vector|VectorLength _returnvalue_3) 0.0)
      (Transformation|SetActorRotation (Math|Conversions|RotationFromXVector _returnvalue_4)) ; Rotate from camera direction
      (Character|LaunchCharacter (+ (* _returnvalue_4 1.2e+03) "0,0.000000,800.000000") true true)
      (else
        (Transformation|SetActorRotation (Math|Rotator|MakeRotator 0.0 0.0 (.Yaw (Math|Rotator|BreakRotator (Math|Conversions|RotationFromXVector _out))))) ; Rotate from movement direction
        (Character|LaunchCharacter (+ (* _returnvalue_3 1.2e+03) "0,0.000000,800.000000") true true)))))

(fn EndDive
  (params (AllowForNewDive :type Boolean))
  (if AllowForNewDive
    (Variables|Dive|SetCanDive true)
    (else
      (Variables|Dive|SetCanDive false)))
  (Variables|Dive|SetDive false)
  (Variables|Default|SetLockMovement false)
  (return))

(fn PerformEndDiveChecks
  (if (AI|Components|NavMovement|IsMovingonGround (Variables|Character|GetCharacterMovement))
    (Dive|EndDive true)))

(fn Die
  (Variables|Default|Setalive false)
  (switch Utilities|FlowControl|Switch|SwitchonEMovesetEnum (Class|PlatformerGameCharacter|GetMoveset)
    (:M_Default
      _)
    (:M_Helicopter
      _)
    (:M_Balloon
      (Audio|Components|Audio|Play (Variables|Default|GetPopSound) 0.0)))
  (Audio|Components|Audio|Play (Variables|Default|GetDeathSound) 0.0))

(fn HandleHeadInflation
  (if (> (Variables|HeadInflation|GetHeadInflation) 0.0)
    (bind _output_get (Variables|HeadInflation|SetHeadInflation (- (Variables|HeadInflation|GetHeadInflation) (* 2e+01 (Utilities|Time|GetWorldDeltaSeconds)))))
    (if (> _output_get (Variables|HeadInflation|GetMaxHeadInflation))
      (Variables|HeadInflation|SetBoyTint (Math|Color|Lerp(LinearColor) "(R=1.000000,G=1.000000,B=1.000000,A=1.000000)" "(R=1.000000,G=0.000000,B=0.000000,A=1.000000)" (/ (Variables|HeadInflation|GetHeadInflation) (Variables|HeadInflation|GetMaxHeadInflation))))
      (return (Variables|HeadInflation|GetHeadInflation))
      (else
        (if (> (Variables|HeadInflation|GetHeadInflation) (Variables|HeadInflation|GetHeadInflationWarning)) ; Flash the red tint
          (bind _output_get_2 (Variables|HeadInflation|SetTintCountdown (- (Variables|HeadInflation|GetTintCountdown) (Utilities|Time|GetWorldDeltaSeconds))))
          (if (< _output_get_2 0.0)
            (Variables|HeadInflation|SetTintCountdown 0.1)
            (Variables|HeadInflation|SetTintFlashFlag (not (Variables|HeadInflation|GetTintFlashFlag)))
            (if (Variables|HeadInflation|GetTintFlashFlag)
              (Variables|HeadInflation|SetBoyTint "(R=1.000000,G=0.000000,B=0.017682,A=1.000000)")
              (else
                (Variables|HeadInflation|SetBoyTint "(R=1.000000,G=1.000000,B=1.000000,A=1.000000)"))))
          (else
            (Variables|HeadInflation|SetBoyTint (Math|Color|Lerp(LinearColor) "(R=1.000000,G=1.000000,B=1.000000,A=1.000000)" "(R=1.000000,G=0.000000,B=0.000000,A=1.000000)" (/ (Variables|HeadInflation|GetHeadInflation) (Variables|HeadInflation|GetMaxHeadInflation))))))
        (return (Variables|HeadInflation|GetHeadInflation))))
    (else
      (return (Variables|HeadInflation|GetHeadInflation)))))