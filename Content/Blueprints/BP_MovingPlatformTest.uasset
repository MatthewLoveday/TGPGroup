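; Test moving platform that shifts its Cube while a Character overlaps it and moves it back toward the start otherwise.
; BeginPlay caches the start and an end point raised on Z, while overlap events toggle the occupancy flag.
; Tick applies a fixed, frame-rate-dependent X step without sweep until the target matches.
; The X-only step never reaches the Z-offset end, so outward travel is unbounded while occupied.
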(event EventBeginPlay
  (bind _cube (Variables|Default|GetCube))
  (bind _returnvalue (Transformation|GetWorldLocation _cube))
  (Variables|Default|SetStartLocation (Transformation|GetWorldLocation (Variables|Default|GetCube)))
  (Variables|Default|SetPlayerOnPlatform false)
  (Variables|Default|SetVecMovementAmount "10.000000, 0,0.000000")
  (Variables|Default|SetEndLocation (Math|Vector|MakeVector (.x _returnvalue) (.y _returnvalue) (+ (.z _returnvalue) 5e+02)))
  (Development|PrintString "Hello"))

(event Collision|EventActorBeginOverlap
  (params (OtherActor :type Actor%20Object%20Reference))
  (Utilities|Casting|CastToCharacter OtherActor)
  (Variables|Default|SetPlayerOnPlatform true)
  (Development|PrintString "player on platform"))

(event EventTick
  (params (DeltaSeconds :type Float%20%28single-precision%29))
  (if (Variables|Default|GetPlayerOnPlatform)
    (if (not (Math|Vector|Equal(Vector) (Transformation|GetWorldLocation (Variables|Default|GetCube)) (Variables|Default|GetEndLocation) 0.0001))
      (Transformation|SetWorldLocation (Variables|Default|GetCube) (+ (Variables|Default|GetVecMovementAmount) (Transformation|GetWorldLocation (Variables|Default|GetCube))) false false))
    (elif (not (Math|Vector|Equal(Vector) (Transformation|GetWorldLocation (Variables|Default|GetCube)) (Variables|Default|GetStartLocation) 0.0001))
      (Transformation|SetWorldLocation (Variables|Default|GetCube) (- (Transformation|GetWorldLocation (Variables|Default|GetCube)) (Variables|Default|GetVecMovementAmount)) false false))))

(event Collision|EventActorEndOverlap
  (params (OtherActor :type Actor%20Object%20Reference))
  (Variables|Default|SetPlayerOnPlatform false)
  (Development|PrintString (Utilities|String|ToString(Boolean) (Variables|Default|GetPlayerOnPlatform))))

(fn ConstructionScript)