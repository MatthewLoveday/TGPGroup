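; Utility Blueprint that toggles the sky between a bright blue look and a dark, cloudy grey one on left mouse click.
; A FlipFlop, gated on a valid SkyRef, alternately plays and reverses one timeline for a smooth transition both ways.
; The timeline's track drives lerps on the sky material's zenith, horizon and cloud parameters, and dims LightRef's color to match.
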(event Input|MouseEvents|LeftMouseButton
  (params (Key :type Key%20Structure))
  (bind _skyref (Variables|Default|GetSkyRef))
  (bind _sky_material (Variables|/Engine/EngineSky/BP_Sky_Sphere.BP_Sky_Sphere_C|GetSky%20material _skyref))
  (:Pressed
    (if (Utilities|IsValid (Variables|Default|GetSkyRef))
      (Utilities|FlowControl|FlipFlop
        (:A
          (bind _newtrack_0 (Timeline|Timeline_0 Play)
            (:Update
              (Rendering|Material|SetVectorParameterValue _sky_material "Zenith color" (Math|Color|Lerp(LinearColor) "(R=0.034046,G=0.109247,B=0.295000,A=1.000000)" "(R=0.156250,G=0.156250,B=0.156250,A=1.000000)" _newtrack_0) :!class /Script/Engine.MaterialInstanceDynamic)
              (Rendering|Material|SetVectorParameterValue _sky_material "Horizon color" (Math|Color|Lerp(LinearColor) "(R=1.979559,G=2.586644,B=3.000000,A=1.000000)" "(R=0.072917,G=0.072917,B=0.072917,A=1.000000)" _newtrack_0) :!class /Script/Engine.MaterialInstanceDynamic)
              (Rendering|Material|SetVectorParameterValue _sky_material "Cloud color" (Math|Color|Lerp(LinearColor) "(R=0.855778,G=0.919020,B=1.000000,A=1.000000)" "(R=0.067708,G=0.067708,B=0.067708,A=1.000000)" _newtrack_0) :!class /Script/Engine.MaterialInstanceDynamic)
              (Rendering|Material|SetScalarParameterValue _sky_material "Cloud opacity" (Math|Float|Lerp 1.2 5.0 _newtrack_0) :!class /Script/Engine.MaterialInstanceDynamic)
              (Rendering|Components|Light|SetLightColor (Variables|/Script/Engine.Light|GetLightComponent (Variables|Default|GetLightRef)) (Math|Color|Lerp(LinearColor) "(R=1.000000,G=1.000000,B=1.000000,A=1.000000)" "(R=0.234375,G=0.234375,B=0.234375,A=1.000000)" _newtrack_0) true))))
        (:B
          (Timeline|Timeline_0 Reverse))))))

(fn ConstructionScript)