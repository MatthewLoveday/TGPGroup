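; Test door actor that swings open in yaw when an actor overlaps it, then swings back to its starting rotation.
; BeginPlay caches start and target transforms, overlap sets the trigger flags, and Tick calls the open or return rotation function.
; Rotation steps a fixed amount per frame, so speed depends on frame rate.
; A vertical raise-and-lower variant exists but never runs, and debug strings print values.
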(event EventBeginPlay
  (bind _returnvalue (Transformation|GetActorLocation))
  (bind _output_get (Variables|Default|SetMovementAmount "0, 0,200.000000"))
  (Variables|Default|SetDistanceToMove (+ _output_get _returnvalue))
  (Variables|Default|SetStartLocation _returnvalue)
  (bind _output_get_2 (Variables|Default|SetRotationAmount "0,90.000000, 0"))
  (Variables|Default|SetDistanceToRotate (Math|Rotator|MakeRotator (.roll _output_get_2) (.pitch _output_get_2) (+ (.yaw _output_get_2) (.yaw (Transformation|GetActorRotation)))))
  (Variables|Default|SetStartRotation (Transformation|GetActorRotation))
  (Development|PrintString (Utilities|String|ToString(Rotator) (Variables|Default|GetDistanceToRotate)) true true "(R=0.000000,G=0.660000,B=1.000000,A=1.000000)" 1e+01)
  (Development|PrintString (Utilities|String|ToString(Rotator) (Variables|Default|GetRotationAmount)) true true "(R=0.000000,G=0.660000,B=1.000000,A=1.000000)" 1e+01)
  (Development|PrintString (Utilities|String|ToString(Rotator) (Variables|Default|GetStartRotation)) true true "(R=0.000000,G=0.660000,B=1.000000,A=1.000000)" 1e+01))

(event Collision|EventActorBeginOverlap
  (params (OtherActor :type Actor%20Object%20Reference))
  (Development|PrintString "Hello")
  (bind _output_get (Variables|Default|SetCanMove true))
  (Development|PrintString (Utilities|String|Append "CanMove: " (Utilities|String|ToString(Boolean) _output_get)))
  (Variables|Default|SetCanRotate true))

(event EventTick
  (params (DeltaSeconds :type Float%20%28single-precision%29))
  (if (Variables|Default|GetCanRotate)
    (CallFunction|RotateDoortoLocation)
    (else
      (CallFunction|RotateDoortoStartLocation))))

(fn ConstructionScript)

(fn MoveDoortoLocation
  (bind _returnvalue (Transformation|GetActorLocation))
  (if (Math|Vector|Equal(Vector) (Transformation|GetActorLocation) (Variables|Default|GetDistanceToMove) 0.0001)
    (Variables|Default|SetCanMove false)
    (else
      (Transformation|SetActorLocation (Math|Vector|MakeVector (.x _returnvalue) (.y _returnvalue) (+ (.z _returnvalue) 1.0)) false false))))

(fn MoveDoortoStartLocation
  (bind _returnvalue (Transformation|GetActorLocation))
  (Variables|Default|SetMoveToStart true)
  (if (Variables|Default|GetMoveToStart)
    (if (Math|Vector|Equal(Vector) (Transformation|GetActorLocation) (Variables|Default|GetStartLocation) 0.0001)
      (Variables|Default|SetMoveToStart false)
      (else
        (Transformation|SetActorLocation (Math|Vector|MakeVector (.x _returnvalue) (.y _returnvalue) (- (.z _returnvalue) 1.0)) false false)))))

(fn RotateDoortoLocation
  (bind _returnvalue (Transformation|GetActorRotation))
  (if (not (>= (.yaw (Transformation|GetActorRotation)) (.yaw (Variables|Default|GetDistanceToRotate))))
    (Transformation|SetActorRotation (Math|Rotator|MakeRotator (.roll _returnvalue) (.pitch _returnvalue) (+ (.yaw _returnvalue) 1.0)))
    (if (>= (.yaw (Transformation|GetActorRotation)) (.yaw (Variables|Default|GetDistanceToRotate)))
      (Variables|Default|SetCanRotate false)
      (Variables|Default|SetRotateToStart true))))

(fn RotateDoortoStartLocation
  (bind _returnvalue (Transformation|GetActorRotation))
  (if (Variables|Default|GetRotateToStart)
    (if (<= (.yaw (Transformation|GetActorRotation)) (.yaw (Variables|Default|GetStartRotation)))
      (Variables|Default|SetRotateToStart false)
      (else
        (Transformation|SetActorRotation (Math|Rotator|MakeRotator (.roll _returnvalue) (.pitch _returnvalue) (- (.yaw _returnvalue) 1.0)))))))