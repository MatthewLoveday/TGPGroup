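; Save point actor that persists the collected state of every BP_PickupBrokenChain in the level.
; Any actor overlap creates a fresh BP_SaveGame, fills its PickupIsCollected array from the pickups and writes slot "Test".
; BeginPlay loads that slot if present and copies each flag back, matching pickups by GetAllActorsOfClass index, so restoration depends on stable actor order.
; Print strings report each step.
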(event EventBeginPlay
  (bind _returnvalue (SaveGame|DoesSaveGameExist "Test"))
  (if _returnvalue
    (Development|PrintString "Save exists")
    (bind _returnvalue_2 (SaveGame|LoadGamefromSlot "Test"))
    (bind _asbp_save_game (Utilities|Casting|CastToBP_SaveGame _returnvalue_2)
      (:then
        (bind _output_get (Variables|Default|SetSaveGameRef _asbp_save_game))
        (bind _outactors (Actor|GetAllActorsOfClass "/Game/Blueprints/Pickups/BP_PickupBrokenChain.BP_PickupBrokenChain_C"))
        (for (_array_element _array_index) _outactors
          (bind _output_get_2 (Variables|/Game/Blueprints/Pickups/BP_PickupBrokenChain.BP_PickupBrokenChain_C|SetIsCollected _array_element (Utilities|Array|Get(acopy) (Variables|/Game/Blueprints/BP_SaveGame.BP_SaveGame_C|GetPickupIsCollected _output_get) _array_index)))
          (Development|PrintString (Utilities|String|ToString(Boolean) _output_get_2))))
      (:CastFailed
        (Development|PrintString "Cast failed")))
    (else
      (Development|PrintString "Save does not exist"))))

(event Collision|EventActorBeginOverlap
  (params (OtherActor :type Actor%20Object%20Reference))
  ;[1 1 1] save the game
  (bind _returnvalue (SaveGame|CreateSaveGameObject "/Game/Blueprints/BP_SaveGame.BP_SaveGame_C"))
  (bind _output_get (Variables|Default|SetSaveGameRef _returnvalue))
  (bind _outactors (Actor|GetAllActorsOfClass "/Game/Blueprints/Pickups/BP_PickupBrokenChain.BP_PickupBrokenChain_C"))
  (for _array_element _outactors
    (Utilities|Array|Add (Variables|/Game/Blueprints/BP_SaveGame.BP_SaveGame_C|GetPickupIsCollected _output_get) (Variables|/Game/Blueprints/Pickups/BP_PickupBrokenChain.BP_PickupBrokenChain_C|GetIsCollected _array_element))
    (Development|PrintString (Utilities|String|ToString(Boolean) (Variables|/Game/Blueprints/Pickups/BP_PickupBrokenChain.BP_PickupBrokenChain_C|GetIsCollected _array_element))))
  (bind _returnvalue_2 (SaveGame|SaveGametoSlot (Variables|Default|GetSaveGameRef) "Test"))
  (if _returnvalue_2
    (Development|PrintString "Save complete")
    (else
      (Development|PrintString "Save failed"))))

(event EventTick
  (params (DeltaSeconds :type Float%20%28single-precision%29)))

(fn ConstructionScript)