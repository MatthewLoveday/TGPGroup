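; BP_PickupBrokenChain is a broken chain pickup that counts toward the player character's BrokenChainCount.
; On overlap it casts the other actor to CharacterBP, increments that count, then prints the character's separate CollectableCount as debug text.
; BeginPlay prints its IsCollected flag, but the graph never sets that flag or destroys the actor, so repeated overlaps keep adding to the count.
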(event EventBeginPlay
  (if true
    (Development|PrintString (Utilities|String|Append "IsCollected" (Utilities|String|ToString(Boolean) (Variables|Default|GetIsCollected))) true true "(R=0.000000,G=0.660000,B=1.000000,A=1.000000)" 1e+01)))

(event Collision|EventActorBeginOverlap
  (params (OtherActor :type Actor%20Object%20Reference))
  (bind _ascharacter_bp (Utilities|Casting|CastToCharacterBP OtherActor))
  (bind _result (Math|Integer|IncrementInt (Variables|/Script/tgp.PlatformerGameCharacter|GetBrokenChainCount _ascharacter_bp))
    (:%20%20
      (Variables|/Script/tgp.PlatformerGameCharacter|SetBrokenChainCount _ascharacter_bp _result)
      (Development|PrintString (Utilities|String|Append "Collectable Count: " (Utilities|String|ToString(Integer) (Variables|/Game/Blueprints/Player/CharacterBP.CharacterBP_C|GetCollectableCount _ascharacter_bp)))))))

(event EventTick
  (params (DeltaSeconds :type Float%20%28single-precision%29)))

(fn ConstructionScript)