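; A sign actor that shows a text popup while the player character stands in its Activator volume.
; BeginPlay creates a TextPrompt widget from TextForPopup, and a CharacterBP entering the volume adds it to the viewport, guarded by an Overlapping flag.
; Any actor leaving clears the flag; if it is a CharacterBP, all widgets are removed and the character's AddUI is called to restore its UI.
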(event OnComponentBeginOverlap(Activator)
  (params (OverlappedComponent :type Primitive%20Component%20Object%20Reference) (OtherActor :type Actor%20Object%20Reference) (OtherComp :type Primitive%20Component%20Object%20Reference) (OtherBodyIndex :type Integer) (bFromSweep :type Boolean) (SweepResult :type Hit%20Result%20Structure%20%28by%20ref%29))
  (if (not (Variables|Default|GetOverlapping))
    (Utilities|Casting|CastToCharacterBP OtherActor)
    (UserInterface|Viewport|AddtoViewport (Variables|Default|GetTextWidget) 0)
    (Variables|Default|SetOverlapping true)))

(event OnComponentEndOverlap(Activator)
  (params (OverlappedComponent :type Primitive%20Component%20Object%20Reference) (OtherActor :type Actor%20Object%20Reference) (OtherComp :type Primitive%20Component%20Object%20Reference) (OtherBodyIndex :type Integer))
  (Variables|Default|SetOverlapping false)
  (bind _ascharacter_bp (Utilities|Casting|CastToCharacterBP OtherActor))
  (Viewport|RemoveAllWidgets)
  (Default|AddUI _ascharacter_bp))

(event EventBeginPlay
  (bind _returnvalue (UserInterface|CreateWidget "/Game/UI/TextPrompt.TextPrompt_C" (Game|GetPlayerController 0)))
  (Variables|/Game/UI/TextPrompt.TextPrompt_C|SetTextValue _returnvalue (Variables|Default|GetTextForPopup))
  (Variables|Default|SetTextWidget _returnvalue))

(event Collision|EventActorBeginOverlap
  (params (OtherActor :type Actor%20Object%20Reference)))

(event EventTick
  (params (DeltaSeconds :type Float%20%28single-precision%29)))

(fn ConstructionScript)