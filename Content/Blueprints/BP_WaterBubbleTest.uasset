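; Test actor for a water bubble that repeatedly rises from its placed location with a sideways wobble.
; BeginPlay stores the start and a top point RiseAmount above it; each Tick, Rise moves it up one unit, frame-rate dependent, and nudges Y by a sine of a counter scaled by delta time.
; On exactly matching the top Z, it waits briefly, then snaps back to the start.
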(event EventBeginPlay
  (bind _returnvalue (Transformation|GetActorLocation))
  (Variables|Default|SetBubbleRisePos (Math|Vector|MakeVector (.x _returnvalue) (.y _returnvalue) (+ (.z _returnvalue) (Variables|Default|GetRise%20amount))))
  (Variables|Default|SetStart%20pos (Transformation|GetActorLocation)))

(event Collision|EventActorBeginOverlap
  (params (OtherActor :type Actor%20Object%20Reference)))

(event EventTick
  (params (DeltaSeconds :type Float%20%28single-precision%29))
  (if (== (.z (Transformation|GetActorLocation)) (.z (Variables|Default|GetBubbleRisePos)))
    (Utilities|FlowControl|Delay 1.0)
    (Transformation|SetActorLocation (Variables|Default|GetStart%20pos) false false)
    (else
      (CallFunction|Rise DeltaSeconds))))

(fn ConstructionScript)

(fn Rise
  (params (DeltaTime :type Float%20%28single-precision%29))
  (bind _returnvalue (Transformation|GetActorLocation))
  (bind _result (Math|Integer|IncrementInt (Variables|Default|GetBounceVal))
    (:%20%20
      (Transformation|SetActorLocation (Math|Vector|MakeVector (.x _returnvalue) (+ (Math|Trig|Sin(Radians) (* _result (* DeltaTime 4.0))) (.y _returnvalue)) (+ (.z _returnvalue) 1.0)) false false))))