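; Test player character for a third-person platformer with camera-relative movement, wall jumping, mid-air diving and dive-jumps.
; Tick runs circle-trace wall checks that drive wall-slide state, gravity changes and an unfinished ledge hang.
; Jump and Dive inputs launch the character based on that state, and a Tick box trace ends dives.
; Tick also adds extra fall gravity and sets animation flags, while foot overlaps puff smoke.
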(event OnComponentBeginOverlap(LeftFoot)
  (params (OverlappedComponent :type Primitive%20Component%20Object%20Reference) (OtherActor :type Actor%20Object%20Reference) (OtherComp :type Primitive%20Component%20Object%20Reference) (OtherBodyIndex :type Integer) (bFromSweep :type Boolean) (SweepResult :type Hit%20Result%20Structure%20%28by%20ref%29))
  (bind _footsmoke (Variables|Default|GetFootSmoke))
  ;[1 1 1] Feet Smoke
  (Components|Activation|Activate _footsmoke true)
  (Utilities|FlowControl|Delay 0.2)
  (Components|Activation|Deactivate _footsmoke))

(event OnComponentBeginOverlap(RightFoot)
  (params (OverlappedComponent :type Primitive%20Component%20Object%20Reference) (OtherActor :type Actor%20Object%20Reference) (OtherComp :type Primitive%20Component%20Object%20Reference) (OtherBodyIndex :type Integer) (bFromSweep :type Boolean) (SweepResult :type Hit%20Result%20Structure%20%28by%20ref%29))
  (bind _footsmoke (Variables|Default|GetFootSmoke))
  ;[1 1 1] Feet Smoke
  (Components|Activation|Activate _footsmoke true)
  (Utilities|FlowControl|Delay 0.2)
  (Components|Activation|Deactivate _footsmoke))

(event EventTick
  (params (DeltaSeconds :type Float%20%28single-precision%29))
  (bind _returnvalue (Transformation|GetActorLocation))
  ;[1 1 1] Tick
  (AnimVariables|UpdateAnimVariables)
  (Debug|DebugDrawMovement (Utilities|DrawDebug))
  (WallJump|PerformWallChecks)
  (CallFunction|DetermineifGroundApproach 4e+02)
  (CallFunction|PerformBetterJump)
  (Variables|/Script/Engine.CharacterMovementComponent|SetbOrientRotationToMovement (Variables|Character|GetCharacterMovement) (not (AI|Components|NavMovement|IsFalling (Variables|Character|GetCharacterMovement))))
  (bind _returnvalue_2 (Collision|BoxTraceByChannel _returnvalue _returnvalue "30.000000,30.000000,150.000000" "0, 0, 0" "TraceTypeQuery4" false 0 "None"))
  (if _returnvalue_2
    (Dive|EndDive)))

(event Input|ActionEvents|InputActionJump
  (params (Key :type Key%20Structure))
  ;[1 1 1] Perform Jump
  (:Pressed
    (if (Variables|WallJump|GetIsOnWall)
      (WallJump|JumpOffWall)
      (else
        (Character|Jump)
        (Dive|TryDiveJump))))
  (:Released
    (Character|StopJumping)))

(event Input|ActionEvents|InputActionDive
  (params (Key :type Key%20Structure))
  ;[1 1 1] Dive
  (:Pressed
    (Dive|TryBeginDive)))

(event Input|AxisEvents|InputAxisForwardMovement
  (params (AxisValue :type Float%20%28single-precision%29))
  ;[1 1 1] Player Movement
  (if (not (Variables|Default|GetLockInput))
    (Pawn|Input|AddMovementInput (Math|Vector|GetForwardVector (Math|Rotator|MakeRotator 0.0 0.0 (.Yaw (Math|Rotator|BreakRotator (Pawn|GetControlRotation :!class /Script/Engine.Pawn))))) AxisValue false)))

(event Input|AxisEvents|InputAxisHorizontalMovement
  (params (AxisValue :type Float%20%28single-precision%29))
  ;[1 1 1] Player Movement
  (if (not (Variables|Default|GetLockInput))
    (Pawn|Input|AddMovementInput (Math|Vector|GetRightVector (Math|Rotator|MakeRotator 0.0 0.0 (.Yaw (Math|Rotator|BreakRotator (Pawn|GetControlRotation :!class /Script/Engine.Pawn))))) AxisValue false)))

(event Input|AxisEvents|InputAxisMouseHorizontal
  (params (AxisValue :type Float%20%28single-precision%29))
  ;[1 1 1] Mouse Movement
  (Pawn|Input|AddControllerYawInput AxisValue))

(event Input|AxisEvents|InputAxisMouseVertical
  (params (AxisValue :type Float%20%28single-precision%29))
  ;[1 1 1] Mouse Movement
  (Pawn|Input|AddControllerPitchInput AxisValue))

(event Input|KeyboardEvents|E
  (params (Key :type Key%20Structure))
  (bind _returnvalue (Transformation|GetActorLocation))
  (:Pressed
    (bind _outhits (Class|KismetSystemLibrary|LineTraceMultiforObjects _returnvalue (+ _returnvalue (* (Math|Vector|GetForwardVector (Math|Conversions|RotationFromXVector _returnvalue)) (Variables|Default|GetDistance))) "ObjectTypeQuery1" false 0 "Persistent" true))
    (for _array_element _outhits
      _)))

(fn ConstructionScript)

(fn UpdateAnimVariables
  (Variables|AnimVariables|SetWalking (or (!= (Input|AxisValues|GetForwardMovement) 0.0) (!= (Input|AxisValues|GetHorizontalMovement) 0.0)))
  (return))

(fn EnterWalljump
  (params (WallNormal :type Vector))
  (bind _charactermovement (Variables|Character|GetCharacterMovement))
  (if (not (Variables|WallJump|GetIsOnWall))
    (Variables|WallJump|SetIsOnWall true)
    (Variables|/Script/Engine.CharacterMovementComponent|SetGravityScale _charactermovement 1.0)
    (Variables|WallJump|SetWallNormal (Math|Vector|Normalize WallNormal))
    (Variables|/Script/Engine.MovementComponent|SetVelocity _charactermovement (Math|Vector|MakeVector (.X (Math|Vector|BreakVector (Variables|/Script/Engine.MovementComponent|GetVelocity _charactermovement))) (.Y (Math|Vector|BreakVector (Variables|/Script/Engine.MovementComponent|GetVelocity _charactermovement))) 0.0))
    (Variables|WallJump|SetWallCooldown 0.5)
    (Components|Activation|Activate (Variables|Default|GetWallSmoke) true)
    (Variables|Dive|SetDive false)
    (return)))

(fn LeaveWallJump
  (if (Variables|WallJump|GetIsOnWall)
    (Variables|WallJump|SetIsOnWall false)
    (Variables|/Script/Engine.CharacterMovementComponent|SetGravityScale (Variables|Character|GetCharacterMovement) 3.0)
    (Variables|WallJump|SetWallCooldown 0.5)
    (Components|Activation|Deactivate (Variables|Default|GetWallSmoke))
    (return)))

(fn GetPlayerPushingTowardVector
  (params (Vector :type Vector) (Threshold :type Float%20%28single-precision%29))
  (return (>= (Math|Vector|DotProduct Vector (Math|Vector|Normalize (+ (Transformation|GetVelocity) (* (VectorHelpers|CalculateMovementVector) 25.0)))) Threshold)))

(fn DebugDrawVelocity
  (params (Length :type Float%20%28single-precision%29) (Draw :type Boolean))
  (bind _returnvalue (Transformation|GetActorLocation))
  (if Draw
    (Rendering|Debug|DrawDebugLine _returnvalue (+ _returnvalue (* (Math|Vector|Normalize (Variables|/Script/Engine.MovementComponent|GetVelocity (Variables|Character|GetCharacterMovement))) Length)) "(R=1.000000,G=0.997690,B=0.962442,A=1.000000)" 0.0 1e+01)
    (return)
    (else
      (return))))

(fn DebugDrawMovement
  (params (Draw :type Boolean))
  (bind _returnvalue (Transformation|GetActorLocation))
  (if Draw
    (Rendering|Debug|DrawDebugLine _returnvalue (+ _returnvalue (* (VectorHelpers|CalculateMovementVector) 2e+02)) "(R=1.000000,G=0.000000,B=0.183393,A=1.000000)" 0.0 1e+01))
  (return))

(fn CalculateMovementVector
  (bind _returnvalue (Pawn|GetControlRotation :!class /Script/Engine.Pawn))
  (bind _yaw (Math|Rotator|BreakRotator _returnvalue))
  (bind _returnvalue_2 (Math|Rotator|MakeRotator 0.0 0.0 _yaw))
  (return (Math|Vector|Normalize (+ (* (Math|Vector|GetForwardVector _returnvalue_2) (Input|AxisValues|GetForwardMovement)) (* (Math|Vector|GetRightVector _returnvalue_2) (Input|AxisValues|GetHorizontalMovement))))))

(fn PerformWallChecks
  (bind _draw_debug (Utilities|DrawDebug))
  ;[1 1 1] If we're next to a wall && not grounded
  (bind _output_get (Variables|WallJump|SetWallCooldown (- (Variables|WallJump|GetWallCooldown) (Utilities|Time|GetWorldDeltaSeconds))))
  (if (<= _output_get 0.0) ; Cooldown to prevent double wall jump
    (if (not (AI|Components|NavMovement|IsFalling (Variables|Character|GetCharacterMovement)))
      (Variables|WallJump|SetWallJumpString? false))
    (Utilities|FlowControl|Sequence
      (:then_0
        (bind _returnvalue (Class|PlatformerGameCharacter|PerformCircleTrace "ECC_GameTraceChannel1" 5e+01 8e+01 _draw_debug))
        (LocalVariables|SetLWallCollide (.bBlockingHit (Collision|BreakHitResult _returnvalue)))
        (LocalVariables|SetLWallNormal (.ImpactNormal (Collision|BreakHitResult _returnvalue))))
      (:then_1
        (bind _returnvalue_2 (Class|PlatformerGameCharacter|PerformCircleTrace "ECC_GameTraceChannel1" 6e+01 8e+01 _draw_debug)) ; Determine if we should hang off the wall
        (LocalVariables|SetLHeadCollide (.bBlockingHit (Collision|BreakHitResult _returnvalue_2))))
      (:then_2
        (if (and (LocalVariables|GetLWallCollide) (LocalVariables|GetLHeadCollide))
          (if (!= (.Z (Math|Vector|BreakVector (LocalVariables|GetLWallNormal))) 1.0)
            (if (AI|Components|NavMovement|IsFalling (Variables|Character|GetCharacterMovement)) ; If the character is in the air
              (bind _result (VectorHelpers|GetPlayerPushingTowardVector (Math|Vector|RotateVector (Math|Vector|MakeVector (.X (Math|Vector|BreakVector (LocalVariables|GetLWallNormal))) (.Y (Math|Vector|BreakVector (LocalVariables|GetLWallNormal))) 0.0) "0,180.000000, 0") 0.25))
              (if (or _result (Variables|WallJump|GetWallJumpString?)) ; If character pushing towards wall
                (WallJump|EnterWalljump (Math|Vector|MakeVector (.X (Math|Vector|BreakVector (LocalVariables|GetLWallNormal))) (.Y (Math|Vector|BreakVector (LocalVariables|GetLWallNormal))) 0.0))
                (return true))
              (else
                (WallJump|LeaveWallJump :!label _label)
                (return false)))
            (else
              (goto _label)))
          (else
            (WallJump|LeaveWallJump)
            (if (and (LocalVariables|GetLWallCollide) (not (LocalVariables|GetLHeadCollide)))
              (Variables|WallJump|SetWallNormal (LocalVariables|GetLWallNormal))
              (CallFunction|BeginHang)
              (else
                (CallFunction|EndHang)))
            (return false)))))))

(fn JumpOffWall
  (bind _wallnormal (Variables|WallJump|GetWallNormal))
  (if (Variables|WallJump|GetIsOnWall)
    (WallJump|LeaveWallJump)
    (Character|LaunchCharacter (* (+ _wallnormal "0, 0,2.000000") 6e+02) true true)
    (Transformation|SetActorRotation (Math|Conversions|RotationFromXVector _wallnormal))
    (Variables|WallJump|SetWallJumpString? true)
    (return)))

(fn PerformBetterJump
  (if (<= (.Z (Math|Vector|BreakVector (Variables|/Script/Engine.MovementComponent|GetVelocity (Variables|Character|GetCharacterMovement)))) 0.0)
    (Variables|/Script/Engine.MovementComponent|SetVelocity (Variables|Character|GetCharacterMovement) (+ (Variables|/Script/Engine.MovementComponent|GetVelocity (Variables|Character|GetCharacterMovement)) (* (* (* "0, 0,1.000000" (Components|Movement|GetGravityZ (Variables|Character|GetCharacterMovement))) (- (Variables|Default|GetFallMultiplier) 1.0)) (Utilities|Time|GetWorldDeltaSeconds))))
    (return)))

(fn DetermineifGroundApproach
  (params (Height :type Float%20%28single-precision%29))
  (bind _returnvalue (Transformation|GetActorLocation))
  (if (<= (.Z (Math|Vector|BreakVector (Variables|/Script/Engine.MovementComponent|GetVelocity (Variables|Character|GetCharacterMovement)))) 0.0)
    (bind _returnvalue_2 (Collision|LineTraceByChannel _returnvalue (+ _returnvalue (Math|Vector|MakeVector 0.0 0.0 (- 0.0 Height))) "TraceTypeQuery1" false 0 "None"))
    (Variables|Dive|SetApproachingGround _returnvalue_2)
    (return)
    (else
      (Variables|Dive|SetApproachingGround false)
      (return))))

(fn TryBeginDive
  (bind _out (VectorHelpers|CalculateMovementVector))
  (bind _returnvalue (Pawn|GetControlRotation :!class /Script/Engine.Pawn))
  (bind _returnvalue_2 (Math|Rotator|GetRotationXVector _returnvalue))
  (bind (_x _y) (Math|Vector|BreakVector _out))
  (bind _returnvalue_3 (Math|Conversions|RotationFromXVector _out))
  (bind (_x_2 _y_2) (Math|Vector|BreakVector _returnvalue_2))
  (bind (_roll _pitch _yaw) (Math|Rotator|BreakRotator _returnvalue_3))
  (bind _returnvalue_4 (Math|Vector|MakeVector _x _y 0.0))
  (if (Math|Boolean|ANDBoolean (AI|Components|NavMovement|IsFalling (Variables|Character|GetCharacterMovement)) (not (Variables|WallJump|GetIsOnWall)) (not (Variables|Dive|GetDive)) (Variables|Dive|GetDiveJumpAvailable))
    (Variables|Dive|SetDive true)
    (Variables|Default|SetLockInput true)
    (if (<= (Math|Vector|VectorLength _returnvalue_4) 0.0)
      (Transformation|SetActorRotation _returnvalue)
      (Character|LaunchCharacter (+ (* (Math|Vector|MakeVector _x_2 _y_2 0.0) 1.2e+03) "0,0.000000,800.000000") true true)
      (else
        (Transformation|SetActorRotation (Math|Rotator|MakeRotator _roll 0.0 _yaw))
        (Character|LaunchCharacter (+ (* _returnvalue_4 1.2e+03) "0,0.000000,800.000000") true true)))))

(fn EndDive
  (Variables|Dive|SetDive false)
  (Variables|Dive|SetDiveJumpAvailable true)
  (Variables|Default|SetLockInput false)
  (return))

(fn TryDiveJump
  (if (and (Variables|Dive|GetDiveJumpAvailable) (Variables|Dive|GetDive))
    (Variables|Dive|SetDive false)
    (Variables|Dive|SetDiveJumpAvailable false)
    (Variables|Default|SetLockInput false)
    (Character|LaunchCharacter (+ (* (VectorHelpers|CalculateMovementVector) 3.5e+02) (Math|Vector|MakeVector 0.0 0.0 (Variables|/Script/Engine.CharacterMovementComponent|GetJumpZVelocity (Variables|Character|GetCharacterMovement)))) true true)
    (Components|Activation|Activate (Variables|Default|GetImpactSmoke) true)
    (Transformation|SetActorRotation (Math|Conversions|RotationFromXVector (VectorHelpers|CalculateMovementVector)))))

(fn BeginHang
  (bind _self self)
  (bind _returnvalue (Transformation|GetActorLocation _self))
  (bind _returnvalue_2 (+ _returnvalue "0, 0,55.000000"))
  (bind _outhit (Collision|LineTraceByChannel _returnvalue_2 (+ _returnvalue_2 (* (Transformation|GetActorForwardVector _self) 6e+01)) "TraceTypeQuery3" false 0 "ForDuration"))
  (if (.bBlockingHit (Collision|BreakHitResult _outhit))
    (Variables|/Script/Engine.CharacterMovementComponent|SetGravityScale (Variables|Character|GetCharacterMovement) 0.0)
    (Transformation|SetActorRotation self (Math|Conversions|RotationFromXVector (.Normal (Collision|BreakHitResult _outhit))))
    (return)))

(fn EndHang
  (Variables|Default|SetHanging false)
  (return))